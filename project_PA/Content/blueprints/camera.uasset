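; An automated screenshot Blueprint that appears meant to capture HDR high-resolution images from a series of camera transforms.
; Tick gathers CineCameraActors, runs an empty console command, takes a screenshot named from text plus an index, then delays one second and loops back to the command.
; The loop that moves an actor through the CameraTransform entries before each capture is disconnected and never runs.
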(event EventTick
  (params (DeltaSeconds :type Float%20%28single-precision%29))
  (Actor|GetAllActorsOfClass "/Script/CinematicCamera.CineCameraActor")
  (Development|ExecuteConsoleCommand "" 0 :!label _label)
  (Class|AutomationBlueprintFunctionLibrary|TakeHighResScreenshot 0 0 (Utilities|String|Append (Variables|Default|Gettext) (Variables|Default|Getindex)) "Literal" false true "High" "" 0.0)
  (Utilities|FlowControl|Delay 1.0)
  (goto _label))

(event EventBeginPlay)

(event Collision|EventActorBeginOverlap
  (params (OtherActor :type Actor%20Object%20Reference)))

(fn ConstructionScript)